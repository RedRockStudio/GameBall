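; Game mode for a ball game that sets up each run and can show the main menu widget.
; On BeginPlay, Game Instance flags trigger Continue or Restart, both spawning a best-distance marker.
; Continue also teleports the ball near its saved position, clears nearby cubes, color switchers and bullets, and repositions "Helper" actors.
; It caches start-to-finish distance for a progress bar; Appodeal ad logic is disconnected, leaving those functions empty.
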(event Custom|CheckContinueEvent
  (bind _playerref (Variables|Default|GetPlayerRef))
  ;[1 1 1] Continue
  (bind _asgb_game_instance (Utilities|Casting|CastToGB_GameInstance (Game|GetGameInstance)))
  (if (Variables|/Game/Blueprints/GB_GameInstance.GB_GameInstance_C|GetContinue? _asgb_game_instance)
    (Variables|/Game/Blueprints/GB_GameInstance.GB_GameInstance_C|SetContinue? _asgb_game_instance false)
    (Physics|SetSimulatePhysics (Variables|/Game/Blueprints/Gameplay/BP_Ball.BP_Ball_C|GetBall _playerref) false)
    (Transformation|SetActorTransform _playerref (Math|Transform|MakeTransform (Math|Vector|MakeVector (- (.x (Variables|/Game/Blueprints/GB_GameInstance.GB_GameInstance_C|GetSavedLocToContinue (Variables|Default|GetGameInstanceRef))) 2.05e+03) 0.0 0.0) "0, 0, 0" "1,1,1") false true)
    (Physics|SetSimulatePhysics (Variables|/Game/Blueprints/Gameplay/BP_Ball.BP_Ball_C|GetBall _playerref) true)
    (Default|SpawnLevelNumberTxt _playerref)
    (CallFunction|SpawnBestDistance)
    (CallFunction|CleanCubesonContinue)
    (CallFunction|SpawnHelpCubes)))

(event Custom|CheckRestartEvent
  ;[1 1 1] Restart
  (bind _asgb_game_instance (Utilities|Casting|CastToGB_GameInstance (Game|GetGameInstance)))
  (if (Variables|/Game/Blueprints/GB_GameInstance.GB_GameInstance_C|GetRestart? _asgb_game_instance)
    (Variables|/Game/Blueprints/GB_GameInstance.GB_GameInstance_C|SetRestart? _asgb_game_instance false)
    (CallFunction|SpawnBestDistance)))

(event Custom|ShowMainWidget
  (bind _returnvalue (Game|GetPlayerController 0))
  ;[1 1 1] Show mainWidget
  (Utilities|IsValid (Variables|Default|GetMainWidgetWB)
    (:Is%20Valid
      _)
    (:Is%20Not%20Valid
      (bind _returnvalue_2 (UserInterface|CreateWidget "/Game/UI/MainWIdget.MainWIdget_C" _returnvalue))
      (Variables|Default|SetMainWidgetWB _returnvalue_2)))
  (UserInterface|Viewport|AddtoViewport (Variables|Default|GetMainWidgetWB) 0)
  (Variables|/Script/Engine.PlayerController|SetbShowMouseCursor _returnvalue true))

(event Custom|AdsBannerShowEvent
  ;[1 1 1] AdsBannerShowEvent
  (CallFunction|AdsShowBanner))

(event EventBeginPlay
  ;[1 1 1] EventBeginPlay
  (bind _outactors (Actor|GetAllActorsOfClass "/Game/Blueprints/Gameplay/BP_Ball.BP_Ball_C"))
  (Variables|Default|SetPlayerRef (Utilities|Array|Get(acopy) _outactors))
  (bind _asgb_game_instance (Utilities|Casting|CastToGB_GameInstance (Game|GetGameInstance)))
  (Variables|Default|SetGameInstanceRef _asgb_game_instance)
  (CallFunction|CheckContinueEvent)
  (CallFunction|CheckRestartEvent)
  (CallFunction|AdsBannerShowEvent) ; Appodeal Banner
  (CallFunction|CheckDistanceforProgressBar))

(fn ConstructionScript)

(fn CleanCubesonContinue
  (Utilities|FlowControl|Sequence
    (:then_0
      ;[1 1 1] Clean Cubes
      (bind _outactors (Actor|GetAllActorsOfClass "/Game/Blueprints/Gameplay/BP_Cube.BP_Cube_C"))
      (for _array_element _outactors
        (if (< (Transformation|GetDistanceTo _array_element (Variables|Default|GetPlayerRef)) (Variables|Default|GetCleanRange))
          (Actor|DestroyActor _array_element))))
    (:then_1
      ;[1 1 1] Clean Color Switchers
      (bind _outactors_2 (Actor|GetAllActorsOfClass "/Game/Blueprints/Gameplay/BP_ColorSwitcher.BP_ColorSwitcher_C"))
      (for _array_element_2 _outactors_2
        (if (< (Transformation|GetDistanceTo _array_element_2 (Variables|Default|GetPlayerRef)) (Variables|Default|GetCleanRange))
          (Actor|DestroyActor _array_element_2))))
    (:then_2
      ;[1 1 1] Clean Bullets
      (bind _outactors_3 (Actor|GetAllActorsOfClass "/Game/Blueprints/Gameplay/BP_Bullet.BP_Bullet_C"))
      (for _array_element_3 _outactors_3
        (if (< (Transformation|GetDistanceTo _array_element_3 (Variables|Default|GetPlayerRef)) (Variables|Default|GetCleanRange))
          (Actor|DestroyActor _array_element_3))))))

(fn SpawnHelpCubes
  (bind _outactors (Actor|GetAllActorswithTag "Helper"))
  (for _array_element _outactors
    (Transformation|SetActorLocation _array_element (Math|Vector|MakeVector (- (.x (Variables|/Game/Blueprints/GB_GameInstance.GB_GameInstance_C|GetSavedLocToContinue (Variables|Default|GetGameInstanceRef))) 4.5e+02) (.y (Transformation|GetActorLocation _array_element)) (.z (Transformation|GetActorLocation _array_element))) false true)))

(fn SpawnBestDistance
  (Game|SpawnActorfromClass "/Game/Blueprints/Gameplay/BP_BestDistance.BP_BestDistance_C" (Math|Transform|MakeTransform (Math|Vector|MakeVector (.x (Variables|/Game/Blueprints/GB_GameInstance.GB_GameInstance_C|GetSavedBestDistance (Variables|Default|GetGameInstanceRef))) 0.0 0.0) "0, 0, 0" "1,1,1") "AlwaysSpawn" 0 0))

(fn AdsShowBanner)

(fn AdsonRestart)

(fn AdsonContinue)

(fn CheckDistanceforProgressBar
  (bind _outactors (Actor|GetAllActorsOfClass "/Script/Engine.PlayerStart"))
  (LocalVariables|SetPlayerStart (Utilities|Array|Get(acopy) _outactors))
  (bind _outactors_2 (Actor|GetAllActorsOfClass "/Game/Blueprints/Gameplay/BP_LevelEnd.BP_LevelEnd_C"))
  (LocalVariables|SetLevelEnd (Utilities|Array|Get(acopy) _outactors_2))
  (Variables|Default|SetDistanceToFinish (- (Transformation|GetDistanceTo (LocalVariables|GetPlayerStart) (LocalVariables|GetLevelEnd)) 4e+02)))