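; BP_Cube is a spinning primitive obstacle that either destroys or reacts physically to a BP_Ball.
; The construction script applies a custom mesh, material and scale, and Tick rotates the actor by SpinPerSecond until movement stops.
; On a hit, a Killer cube destroys the ball.
; Otherwise any hit enables physics and gravity and stops the spin, while a ball hit also adds an impulse along the hit normal.
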(event OnComponentHit(Mesh)
  (params (HitComponent :type Primitive%20Component%20Object%20Reference) (OtherActor :type Actor%20Object%20Reference) (OtherComp :type Primitive%20Component%20Object%20Reference) (NormalImpulse :type Vector :default "0, 0, 0") (Hit :type Hit%20Result%20Structure%20%28by%20ref%29))
  (bind _mesh (Variables|Default|GetMesh))
  (if (Variables|Default|GetKiller?)
    (bind _asbp_ball (Utilities|Casting|CastToBP_Ball OtherActor))
    (Actor|DestroyActor _asbp_ball)
    (else
      (Utilities|FlowControl|Sequence
        (:then_0
          (Physics|SetSimulatePhysics _mesh true)
          (Physics|SetEnableGravity _mesh true)
          (Variables|Default|SetStopMovement? true))
        (:then_1
          (Utilities|Casting|CastToBP_Ball OtherActor)
          (Physics|AddImpulse _mesh (* (.Normal (Collision|BreakHitResult Hit)) 2e+03) "None" false))))))

(event EventTick
  (params (DeltaSeconds :type Float%20%28single-precision%29))
  (bind _spinpersecond (Variables|Default|GetSpinPerSecond))
  (bind _returnvalue (* _spinpersecond DeltaSeconds))
  (if (not (Variables|Default|GetStopMovement?))
    (Transformation|AddActorLocalRotation (Math|Rotator|MakeRotator (.x _returnvalue) (.y _returnvalue) (.z _returnvalue)) false false)))

(fn ConstructionScript
  (bind _mesh (Variables|Default|GetMesh))
  (Components|StaticMesh|SetStaticMesh _mesh (Variables|Default|GetCustomMesh))
  (Rendering|Material|SetMaterial _mesh 0 (Variables|Default|GetCustomMaterial))
  (Transformation|SetRelativeScale3D _mesh (Variables|Transform|GetScaleOffset)))