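; Game mode for the ball game that picks the color scheme on BeginPlay.
; It reuses the index stored in GB_GameInstance if a selection is active, otherwise rolls a random one and saves it there so later loads keep it.
; That index reads parallel ColorsInfo arrays into ball-game color, road and background variables, then fires the OnColorsSelected dispatcher and prints the index.
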(event Custom|ColorPickEvent
  (bind _returnvalue (Game|GetGameInstance))
  (bind _colorsinfo (Variables|Default|GetColorsInfo))
  (bind (_color1 _color2 _roadcolor1 _roadcolor2 _backcolor) (Utilities|Struct|BreakColorsStructure _colorsinfo))
  (bind _asgb_game_instance (Utilities|Casting|CastToGB_GameInstance _returnvalue))
  (bind _asgb_game_instance_2 (Utilities|Casting|CastToGB_GameInstance (Game|GetGameInstance)))
  (if (Variables|/Game/Blueprints/GB_GameInstance.GB_GameInstance_C|GetColorSelectionActivated _asgb_game_instance_2)
    (Variables|Default|SetSelectedColorIndex (Variables|/Game/Blueprints/GB_GameInstance.GB_GameInstance_C|GetSelectedColorIndex (.AsGB%20Game%20Instance (Utilities|Casting|CastToGB_GameInstance (Game|GetGameInstance)))))
    (else
      (Variables|Default|SetSelectedColorIndex (Math|Random|RandomIntegerinRange 0 (Utilities|Array|LastIndex (.Color1 (Utilities|Struct|BreakColorsStructure (Variables|Default|GetColorsInfo))))))))
  (Variables|SelectedColor|SetColor1 (Utilities|Array|Get(acopy) _color1 (Variables|Default|GetSelectedColorIndex)))
  (Variables|SelectedColor|SetColor2 (Utilities|Array|Get(acopy) _color2 (Variables|Default|GetSelectedColorIndex)))
  (Variables|SelectedColor|SetRoadColor1 (Utilities|Array|Get(acopy) _roadcolor1 (Variables|Default|GetSelectedColorIndex)))
  (Variables|SelectedColor|SetRoadColor2 (Utilities|Array|Get(acopy) _roadcolor2 (Variables|Default|GetSelectedColorIndex)))
  (Variables|SelectedColor|SetBackColor (Utilities|Array|Get(acopy) _backcolor (Variables|Default|GetSelectedColorIndex)))
  (Variables|/Game/Blueprints/GB_GameInstance.GB_GameInstance_C|SetColorSelectionActivated _asgb_game_instance true)
  (Variables|/Game/Blueprints/GB_GameInstance.GB_GameInstance_C|SetSelectedColorIndex _asgb_game_instance (Variables|Default|GetSelectedColorIndex))
  (Default|CallOnColorsSelected)
  (Development|PrintString (Utilities|String|ToString(Integer) (Variables|Default|GetSelectedColorIndex))))

(event EventBeginPlay
  (CallFunction|ColorPickEvent))

(fn ConstructionScript)