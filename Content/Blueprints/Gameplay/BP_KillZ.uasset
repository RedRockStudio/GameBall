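; BP_KillZ is a kill volume that removes cubes and kills the player ball when they enter its box.
; On overlap, it calls DestroyCube on any BP_Cube.
; For a BP_Ball, only the component named "Ball" counts, and only while the player can be killed.
; It then flags the player dead and calls the death function on the gameBallGM game mode cached at BeginPlay.
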(event OnComponentBeginOverlap(Box)
  (params (OverlappedComponent :type Primitive%20Component%20Object%20Reference) (OtherActor :type Actor%20Object%20Reference) (OtherComp :type Primitive%20Component%20Object%20Reference) (OtherBodyIndex :type Integer) (bFromSweep :type Boolean) (SweepResult :type Hit%20Result%20Structure%20%28by%20ref%29))
  (Utilities|FlowControl|Sequence
    (:then_0
      (bind _asbp_cube (Utilities|Casting|CastToBP_Cube OtherActor))
      (Default|DestroyCube _asbp_cube))
    (:then_1
      (bind _asbp_ball (Utilities|Casting|CastToBP_Ball OtherActor))
      (if (Utilities|Enum|Equal(Enum) (Utilities|GetObjectName OtherComp) "Ball")
        (if (Variables|/Game/Blueprints/Gameplay/BP_Ball.BP_Ball_C|GetisPlayerCanBeKilled? _asbp_ball)
          (Variables|/Game/Blueprints/Gameplay/BP_Ball.BP_Ball_C|SetisPlayerDead? _asbp_ball true)
          (Default|CallOnPlayerDeath (Variables|Default|GetGameModeRef)))))))

(event EventBeginPlay
  (bind _asgame_ball_gm (Utilities|Casting|CastTogameBallGM (Game|GetGameMode)))
  (Variables|Default|SetGameModeRef _asgame_ball_gm))

(fn ConstructionScript)