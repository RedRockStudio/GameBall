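; Color-coded cube obstacle that kills the player when the ball hits it with a mismatched color tag.
; Construction applies configurable mesh, scale, mass and dynamic material; colors come from the GameInstance, and ColorSwitch flips color and tag.
; It spins on Tick and oscillates between two offsets by timeline until first hit enables physics, with impulse from BP_Ball and sounds on hard impacts.
; DestroyCube freezes physics and shrinks the cube before destroying it.
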(event OnComponentHit(Mesh)
  (params (HitComponent :type Primitive%20Component%20Object%20Reference) (OtherActor :type Actor%20Object%20Reference) (OtherComp :type Primitive%20Component%20Object%20Reference) (NormalImpulse :type Vector :default "0, 0, 0") (Hit :type Hit%20Result%20Structure%20%28by%20ref%29))
  (bind (_bblockinghit _binitialoverlap _time _distance _location _impactpoint _normal _impactnormal _physmat _hitactor _hitcomponent) (Collision|BreakHitResult Hit))
  (bind _mesh (Variables|Default|GetMesh))
  ;[1 1 1] Hit
  (if (not (Variables|Default|GetStopPhysics?))
    (Variables|HitResult|SetNormalImpulse NormalImpulse)
    (Variables|Default|SetHitLocation _location)
    (Variables|HitResult|SetNormal _normal)
    (Variables|HitResult|SetHitComponent _hitcomponent)
    (Utilities|FlowControl|Sequence
      (:then_0
        (Utilities|FlowControl|DoOnce false
          (:Completed
            (Physics|SetSimulatePhysics _mesh true)
            (Physics|SetEnableGravity _mesh true)
            (Variables|Default|SetStopMovement? true)
            (CallFunction|StopMovementEvent))))
      (:then_1
        (bind _asbp_ball (Utilities|Casting|CastToBP_Ball OtherActor))
        (Variables|Default|SetPlayerRef _asbp_ball)
        (Physics|AddImpulse _mesh (* (Variables|HitResult|GetNormal) 2e+02) "None" true)
        (if (Utilities|Enum|Equal(Enum) (Utilities|GetObjectName (Variables|HitResult|GetHitComponent)) "Ball")
          (Utilities|FlowControl|Sequence
            (:then_0
              (if (Utilities|Name|NotEqual(Name) (Utilities|Array|Get(acopy) (Variables|Actor|GetTags self)) (Utilities|Array|Get(acopy) (Variables|/Script/Engine.ActorComponent|GetComponentTags (Variables|HitResult|GetHitComponent))))
                (Utilities|FlowControl|DoOnce false
                  (:Completed
                    (Default|CallOnPlayerDeath (Variables|Default|GetGameModeRef))))))
            (:then_1
              (if (> (Math|Vector|VectorLength (Variables|HitResult|GetNormalImpulse)) 1.5e+04)
                (Utilities|IsValid (Variables|/Game/Blueprints/Gameplay/BP_Ball.BP_Ball_C|GetBall (Variables|Default|GetPlayerRef))
                  (:Is%20Valid
                    (CallFunction|HitSndFunc))))))))
      (:then_2
        (if (and (Utilities|Enum|NotEqual(Enum) (Utilities|GetObjectName (Variables|HitResult|GetHitComponent)) "BoxBallCollision") (> (Math|Vector|VectorLength (Variables|HitResult|GetNormalImpulse)) 1.5e+04))
          (Utilities|IsValid (Variables|/Game/Blueprints/Gameplay/BP_Ball.BP_Ball_C|GetBall (Variables|Default|GetPlayerRef))
            (:Is%20Valid
              (CallFunction|HitSndFunc))))))))

(event Custom|SetCubeColorEvent
  ;[1 1 1] SetColorEvent
  (if (Utilities|Enum|Equal(Enum) (Variables|Default|GetChooseColor) "NewEnumerator0")
    (Rendering|Material|SetVectorParameterValue (Variables|Default|GetDynMat2) "ColorPick2" (Variables|/Game/Blueprints/GB_GameInstance.GB_GameInstance_C|GetColor1 (Variables|Default|GetGameInstanceRef)) :!class /Script/Engine.MaterialInstanceDynamic)
    (else
      (Rendering|Material|SetVectorParameterValue (Variables|Default|GetDynMat2) "ColorPick2" (Variables|/Game/Blueprints/GB_GameInstance.GB_GameInstance_C|GetColor2 (Variables|Default|GetGameInstanceRef)) :!class /Script/Engine.MaterialInstanceDynamic))))

(event Custom|DestroyCube
  (bind _mesh (Variables|Default|GetMesh))
  ;[1 1 1] Destroy Cube
  (Utilities|FlowControl|DoOnce false
    (:Completed
      (Variables|Default|SetStopPhysics? true)
      (Physics|SetSimulatePhysics (Variables|Default|GetMesh) false)
      (bind _tl_scale (Timeline|TL_Scale PlayFromStart)
        (:Update
          (Transformation|SetWorldScale3D _mesh (Math|Vector|Lerp(Vector) (Transformation|GetWorldScale _mesh) "0.010000,0.010000,0.010000" _tl_scale)))
        (:Finished
          (Actor|DestroyActor))))))

(event Custom|RotationEvent
  (params (DeltaSeconds :type Float%20%28single-precision%29))
  (bind _spinpersecond (Variables|Transform|GetSpinPerSecond))
  (bind _returnvalue (* _spinpersecond DeltaSeconds))
  ;[1 1 1] Movements
  (if (not (or (Variables|Default|GetStopMovement?) (Math|Vector|Equal(Vector) (Variables|Transform|GetSpinPerSecond) "0, 0, 0" 0.5)))
    (Transformation|AddActorLocalRotation (Math|Rotator|MakeRotator (.x _returnvalue) (.y _returnvalue) (.z _returnvalue)) false false)))

(event Custom|HitBeginEvent
  (bind _mesh (Variables|Default|GetMesh))
  ;[1 1 1] Hit
  (if (not (Variables|Default|GetStopPhysics?))
    (Variables|HitResult|SetNormalImpulse (stale OnComponentHit(Mesh) NormalImpulse))
    (Variables|Default|SetHitLocation (.Location (Collision|BreakHitResult (stale OnComponentHit(Mesh) Hit))))
    (Variables|HitResult|SetNormal (.Normal (Collision|BreakHitResult (stale OnComponentHit(Mesh) Hit))))
    (Variables|HitResult|SetHitComponent (.HitComponent (Collision|BreakHitResult (stale OnComponentHit(Mesh) Hit))))
    (Utilities|FlowControl|Sequence
      (:then_0
        (Utilities|FlowControl|DoOnce false
          (:Completed
            (Physics|SetSimulatePhysics _mesh true)
            (Physics|SetEnableGravity _mesh true)
            (Variables|Default|SetStopMovement? true)
            (CallFunction|StopMovementEvent))))
      (:then_1
        (bind _asbp_ball (Utilities|Casting|CastToBP_Ball (stale OnComponentHit(Mesh) OtherActor)))
        (Variables|Default|SetPlayerRef _asbp_ball)
        (Physics|AddImpulse _mesh (* (Variables|HitResult|GetNormal) 2e+02) "None" true)
        (if (Utilities|Enum|Equal(Enum) (Utilities|GetObjectName (Variables|HitResult|GetHitComponent)) "Ball")
          (Utilities|FlowControl|Sequence
            (:then_0
              (if (Utilities|Name|NotEqual(Name) (Utilities|Array|Get(acopy) (Variables|Actor|GetTags self)) (Utilities|Array|Get(acopy) (Variables|/Script/Engine.ActorComponent|GetComponentTags (Variables|HitResult|GetHitComponent))))
                (Utilities|FlowControl|DoOnce false
                  (:Completed
                    (Default|CallOnPlayerDeath (Variables|Default|GetGameModeRef))))))
            (:then_1
              (if (> (Math|Vector|VectorLength (Variables|HitResult|GetNormalImpulse)) 1.5e+04)
                (Utilities|IsValid (Variables|/Game/Blueprints/Gameplay/BP_Ball.BP_Ball_C|GetBall (Variables|Default|GetPlayerRef))
                  (:Is%20Valid
                    (CallFunction|HitSndFunc))))))))
      (:then_2
        (if (and (Utilities|Enum|NotEqual(Enum) (Utilities|GetObjectName (Variables|HitResult|GetHitComponent)) "BoxBallCollision") (> (Math|Vector|VectorLength (Variables|HitResult|GetNormalImpulse)) 1.5e+04))
          (Utilities|IsValid (Variables|/Game/Blueprints/Gameplay/BP_Ball.BP_Ball_C|GetBall (Variables|Default|GetPlayerRef))
            (:Is%20Valid
              (CallFunction|HitSndFunc))))))))

(event Custom|PositionMovementEvent
  ;[1 1 1] Movements
  (Variables|Transform|SetMeshCurrLocation (Transformation|GetWorldLocation (Variables|Default|GetMesh)))
  (if (not (and (Math|Vector|Equal(Vector) (Variables|Transform|GetOffsetLocation1) "0, 0, 0" 0.01) (Math|Vector|Equal(Vector) (Variables|Transform|GetOffsetLocation2) "0, 0, 0" 0.01)))
    (Utilities|FlowControl|Sequence
      (:then_0
        (Components|Timeline|SetPlaybackPosition (Variables|Default|GetTL_Offset) (Math|Float|Clamp(Float) (Variables|Transform|GetPlayPosition)) true false)
        (bind _sintrack (Timeline|TL_Offset Play)
          (:Update
            (Components|Timeline|SetPlayRate (Variables|Default|GetTL_Offset) (Variables|Transform|GetNewPlayRate))
            (Components|MoveComponentTo (Variables|Default|GetMesh) (Math|Vector|Lerp(Vector) (+ (Variables|Transform|GetMeshCurrLocation) (Variables|Transform|GetOffsetLocation1)) (+ (Variables|Transform|GetMeshCurrLocation) (Variables|Transform|GetOffsetLocation2)) (Math|Float|Clamp(Float) _sintrack)) (Transformation|GetWorldRotation (Variables|Default|GetMesh)) false false 0.0 false)))))))

(event Custom|StopMovementEvent
  (bind _meshcurrlocation (Variables|Transform|GetMeshCurrLocation))
  ;[1 1 1] Movements
  (bind _sintrack (Timeline|TL_Offset Stop)
    (:Update
      (Components|Timeline|SetPlayRate (Variables|Default|GetTL_Offset) (Variables|Transform|GetNewPlayRate))
      (Components|MoveComponentTo (Variables|Default|GetMesh) (Math|Vector|Lerp(Vector) (+ _meshcurrlocation (Variables|Transform|GetOffsetLocation1)) (+ _meshcurrlocation (Variables|Transform|GetOffsetLocation2)) (Math|Float|Clamp(Float) _sintrack)) (Transformation|GetWorldRotation (Variables|Default|GetMesh)) false false 0.0 false))))

(event EventBeginPlay
  ;[1 1 1] EventBeginPlay
  (Utilities|FlowControl|Sequence
    (:then_0
      (bind _asgb_game_instance (Utilities|Casting|CastToGB_GameInstance (Game|GetGameInstance)))
      (Variables|Default|SetGameInstanceRef _asgb_game_instance)
      (CallFunction|PositionMovementEvent))
    (:then_1
      (bind _asgame_ball_gm (Utilities|Casting|CastTogameBallGM (Game|GetGameMode)))
      (Variables|Default|SetGameModeRef _asgame_ball_gm)
      (CallFunction|SetCubeColorEvent))
    (:then_2
      (bind _outactors (Actor|GetAllActorsOfClass "/Game/Blueprints/Gameplay/BP_Ball.BP_Ball_C"))
      (Variables|Default|SetPlayerRef (Utilities|Array|Get(acopy) _outactors)))))

(event EventTick
  (params (DeltaSeconds :type Float%20%28single-precision%29))
  ;[1 1 1] EventTick
  (CallFunction|RotationEvent DeltaSeconds))

(fn ConstructionScript
  (bind _self self)
  (bind _mesh (Variables|Default|GetMesh))
  (bind _tags (Variables|Actor|GetTags _self))
  (bind _output (Utilities|Array|Get(acopy) _tags))
  (Components|StaticMesh|SetStaticMesh _mesh (Variables|Default|GetCustomMesh))
  (Rendering|Material|SetMaterial _mesh 0 (Variables|Default|GetCustomMaterial))
  (Transformation|SetRelativeScale3D _mesh (Variables|Transform|GetScaleOffset))
  (Class|PrimitiveComponent|SetMassOverrideinKg _mesh "None" (Variables|Default|GetMassKg) true)
  (bind _returnvalue (Rendering|Material|CreateDynamicMaterialInstance _mesh 0 (Variables|Default|GetCustomMaterial) "None" :!class /Script/Engine.PrimitiveComponent))
  (Variables|Default|SetDynMat2 _returnvalue)
  (switch Utilities|FlowControl|Switch|SwitchonShapeTypes (Variables|Default|GetChooseColor)
    (:NewEnumerator0
      (|SetBy-RefVar _output "Color1")
      (Rendering|Material|SetVectorParameterValue (Variables|Default|GetDynMat2) "ColorPick2" "(R=1.000000,G=1.000000,B=1.000000,A=1.000000)" :!class /Script/Engine.MaterialInstanceDynamic))
    (:NewEnumerator1
      (|SetBy-RefVar _output "Color2")
      (Rendering|Material|SetVectorParameterValue (Variables|Default|GetDynMat2) "ColorPick2" "(R=1.000000,G=0.000000,B=0.000000,A=1.000000)" :!class /Script/Engine.MaterialInstanceDynamic))))

(fn ColorSwitch
  (bind _self self)
  (bind _tags (Variables|Actor|GetTags _self))
  (bind _output (Utilities|Array|Get(acopy) _tags))
  (if (Utilities|Name|Equal(Name) (Utilities|Array|Get(acopy) (Variables|Actor|GetTags self)) "Color1")
    (Rendering|Material|SetVectorParameterValue (Variables|Default|GetDynMat2) "ColorPick2" (Variables|/Game/Blueprints/GB_GameInstance.GB_GameInstance_C|GetColor2 (Variables|Default|GetGameInstanceRef)) :!class /Script/Engine.MaterialInstanceDynamic)
    (|SetBy-RefVar _output "Color2")
    (else
      (Rendering|Material|SetVectorParameterValue (Variables|Default|GetDynMat2) "ColorPick2" (Variables|/Game/Blueprints/GB_GameInstance.GB_GameInstance_C|GetColor1 (Variables|Default|GetGameInstanceRef)) :!class /Script/Engine.MaterialInstanceDynamic)
      (|SetBy-RefVar _output "Color1"))))

(fn HitSndFunc
  (Audio|PlaySoundatLocation "/Game/Audio/SndFX/Hit1_Cue.Hit1_Cue" (Variables|Default|GetHitLocation) "0, 0, 0" (Utilities|DistanceBetweenBallandSelf) (Class|Actor|GetActorTimeDilation) 0.0 0 0 0))