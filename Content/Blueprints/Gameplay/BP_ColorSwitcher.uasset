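; Color switcher gate actor that flips the color of a ball or cube passing through it.
; The construction script creates dynamic materials for two meshes and a barrier.
; On BeginPlay it tints them with Color1 and Color2 from GB_GameInstance, making the meshes emissive.
; When an overlap with its box ends, it calls the switch function on BP_Ball (only for the component named "Ball") or BP_Cube.
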(event OnComponentEndOverlap(Box)
  (params (OverlappedComponent :type Primitive%20Component%20Object%20Reference) (OtherActor :type Actor%20Object%20Reference) (OtherComp :type Primitive%20Component%20Object%20Reference) (OtherBodyIndex :type Integer))
  (Utilities|FlowControl|Sequence
    (:then_0
      (bind _asbp_ball (Utilities|Casting|CastToBP_Ball OtherActor))
      (if (Utilities|Enum|Equal(Enum) (Utilities|GetObjectName OtherComp) "Ball")
        (Default|BallColorSwitch _asbp_ball)))
    (:then_1
      (bind _asbp_cube (Utilities|Casting|CastToBP_Cube OtherActor))
      (Default|ColorSwitch _asbp_cube))))

(event Custom|SetColorsEvents
  (bind _barierdynmat (Variables|Default|GetBarierDynMat))
  (bind _asgb_game_instance (Utilities|Casting|CastToGB_GameInstance (Game|GetGameInstance)))
  (Utilities|FlowControl|Sequence
    (:then_0
      (Rendering|Material|SetVectorParameterValue (Variables|Default|GetMesh1DynMat1) "ColorPick2" (Variables|/Game/Blueprints/GB_GameInstance.GB_GameInstance_C|GetColor1 _asgb_game_instance) :!class /Script/Engine.MaterialInstanceDynamic)
      (Rendering|Material|SetScalarParameterValue (Variables|Default|GetMesh1DynMat1) "EmissivePower" 4.0 :!class /Script/Engine.MaterialInstanceDynamic)
      (Rendering|Material|SetVectorParameterValue (Variables|Default|GetMesh1DynMat2) "ColorPick2" (Variables|/Game/Blueprints/GB_GameInstance.GB_GameInstance_C|GetColor2 _asgb_game_instance) :!class /Script/Engine.MaterialInstanceDynamic)
      (Rendering|Material|SetScalarParameterValue (Variables|Default|GetMesh1DynMat2) "EmissivePower" 4.0 :!class /Script/Engine.MaterialInstanceDynamic))
    (:then_1
      (Rendering|Material|SetVectorParameterValue (Variables|Default|GetMesh2DynMat1) "ColorPick2" (Variables|/Game/Blueprints/GB_GameInstance.GB_GameInstance_C|GetColor1 _asgb_game_instance) :!class /Script/Engine.MaterialInstanceDynamic)
      (Rendering|Material|SetScalarParameterValue (Variables|Default|GetMesh2DynMat1) "EmissivePower" 4.0 :!class /Script/Engine.MaterialInstanceDynamic)
      (Rendering|Material|SetVectorParameterValue (Variables|Default|GetMesh2DynMat2) "ColorPick2" (Variables|/Game/Blueprints/GB_GameInstance.GB_GameInstance_C|GetColor2 _asgb_game_instance) :!class /Script/Engine.MaterialInstanceDynamic)
      (Rendering|Material|SetScalarParameterValue (Variables|Default|GetMesh2DynMat2) "EmissivePower" 4.0 :!class /Script/Engine.MaterialInstanceDynamic))
    (:then_2
      (Rendering|Material|SetVectorParameterValue _barierdynmat "ColorPick1" (Variables|/Game/Blueprints/GB_GameInstance.GB_GameInstance_C|GetColor1 _asgb_game_instance) :!class /Script/Engine.MaterialInstanceDynamic)
      (Rendering|Material|SetVectorParameterValue _barierdynmat "ColorPick2" (Variables|/Game/Blueprints/GB_GameInstance.GB_GameInstance_C|GetColor2 _asgb_game_instance) :!class /Script/Engine.MaterialInstanceDynamic))))

(event EventBeginPlay
  (CallFunction|SetColorsEvents))

(fn ConstructionScript
  (Utilities|FlowControl|Sequence
    (:then_0
      (bind _returnvalue (Rendering|Material|CreateDynamicMaterialInstance (Variables|Default|GetCS_Mesh1) 0 "/Game/Materials/MI_Gradient1.MI_Gradient1" "None" :!class /Script/Engine.PrimitiveComponent))
      (Variables|Default|SetMesh1DynMat1 _returnvalue)
      (bind _returnvalue_2 (Rendering|Material|CreateDynamicMaterialInstance (Variables|Default|GetCS_Mesh1) 1 "/Game/Materials/MI_Gradient2.MI_Gradient2" "None" :!class /Script/Engine.PrimitiveComponent))
      (Variables|Default|SetMesh1DynMat2 _returnvalue_2))
    (:then_1
      (bind _returnvalue_3 (Rendering|Material|CreateDynamicMaterialInstance (Variables|Default|GetCS_Mesh2) 0 "/Game/Materials/MI_Gradient1.MI_Gradient1" "None" :!class /Script/Engine.PrimitiveComponent))
      (Variables|Default|SetMesh2DynMat1 _returnvalue_3)
      (bind _returnvalue_4 (Rendering|Material|CreateDynamicMaterialInstance (Variables|Default|GetCS_Mesh2) 1 "/Game/Materials/MI_Gradient2.MI_Gradient2" "None" :!class /Script/Engine.PrimitiveComponent))
      (Variables|Default|SetMesh2DynMat2 _returnvalue_4))
    (:then_2
      (bind _returnvalue_5 (Rendering|Material|CreateDynamicMaterialInstance (Variables|Default|GetCS_Barier) 0 "/Game/Materials/MI_Barier.MI_Barier" "None" :!class /Script/Engine.PrimitiveComponent))
      (Variables|Default|SetBarierDynMat _returnvalue_5))))