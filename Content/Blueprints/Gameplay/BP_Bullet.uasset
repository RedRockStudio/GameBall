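; BP_Bullet is a shooter actor that repeatedly fires cube projectiles along its Arrow component.
; BeginPlay waits an initial delay, then loops: ShootFunc spawns a BP_CubeBullet at the arrow transform, pushes its mesh forward with a large impulse and triggers its HitBeginEvent.
; After a second delay it destroys that bullet through the stored reference and fires again, so each shot lives one interval.
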(event EventBeginPlay
  (Utilities|FlowControl|Delay (Variables|Default|GetFirstDelayTime))
  (CallFunction|ShootFunc :!label _label)
  (Utilities|FlowControl|Delay (Variables|Default|GetdelayTime))
  (Default|DestroyCube (Variables|Default|GetBP_CubeBulletRef))
  (goto _label))

(fn ConstructionScript)

(fn ShootFunc
  (bind _arrow (Variables|Default|GetArrow))
  (bind _returnvalue (Game|SpawnActorfromClass "/Game/Blueprints/Gameplay/BP_CubeBullet.BP_CubeBullet_C" (Transformation|GetWorldTransform _arrow) "Undefined" 0 0))
  (bind _output_get (Variables|Default|SetBP_CubeBulletRef _returnvalue))
  (Physics|AddImpulse (Variables|/Game/Blueprints/Gameplay/BP_CubeBullet.BP_CubeBullet_C|GetMesh _output_get) (* (Math|Vector|GetForwardVector _arrow) 1.5e+05) "None" false)
  (Default|HitBeginEvent _returnvalue))