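; BP_Sky is a sky sphere Blueprint that takes its color from the game mode's background color.
; The construction script creates a dynamic material instance on the sky sphere mesh.
; BeginPlay binds to gameBallGM's OnColorsSelected event.
; SetSkyColorEvent reads BackColor from that game mode and writes it to the material's ColorPick parameter.
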(event Custom|SetSkyColorEvent
  (bind _asgame_ball_gm (Utilities|Casting|CastTogameBallGM (Game|GetGameMode)))
  (Rendering|Material|SetVectorParameterValue (Variables|Default|GetDynMatSky) "ColorPick" (Variables|/Game/Blueprints/Gameplay/gameBallGM.gameBallGM_C|GetBackColor _asgame_ball_gm) :!class /Script/Engine.MaterialInstanceDynamic))

(event EventBeginPlay
  (bind _asgame_ball_gm (Utilities|Casting|CastTogameBallGM (Game|GetGameMode)))
  (EventDispatchers|BindEventtoOnColorsSelected _asgame_ball_gm (EventDispatchers|CreateEvent :!event Custom|SetSkyColorEvent)))

(fn ConstructionScript
  (bind _sky_sphere_mesh (Variables|BP_Skydome|GetSky%20Sphere%20mesh))
  (bind _returnvalue (Rendering|Material|CreateDynamicMaterialInstance _sky_sphere_mesh 0 (Rendering|Material|GetMaterial _sky_sphere_mesh 0) "None" :!class /Script/Engine.PrimitiveComponent))
  (Variables|Default|SetDynMatSky _returnvalue))