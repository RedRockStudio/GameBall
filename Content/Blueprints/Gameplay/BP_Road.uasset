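; BP_Road is a road piece whose two material slots are tinted with colours stored in the game instance.
; The construction script applies a configurable mesh and creates a dynamic material instance for each slot.
; On BeginPlay, SetRoadColorsEvent reads RoadColor1 and RoadColor2 from GB_GameInstance and writes them to each instance's ColorPick parameter.
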(event Custom|SetRoadColorsEvent
  (bind _asgb_game_instance (Utilities|Casting|CastToGB_GameInstance (Game|GetGameInstance)))
  (Rendering|Material|SetVectorParameterValue (Variables|Default|GetDynMatColor1) "ColorPick" (Variables|/Game/Blueprints/GB_GameInstance.GB_GameInstance_C|GetRoadColor1 _asgb_game_instance) :!class /Script/Engine.MaterialInstanceDynamic)
  (Rendering|Material|SetVectorParameterValue (Variables|Default|GetDynMatColor2) "ColorPick" (Variables|/Game/Blueprints/GB_GameInstance.GB_GameInstance_C|GetRoadColor2 _asgb_game_instance) :!class /Script/Engine.MaterialInstanceDynamic))

(event EventBeginPlay
  (CallFunction|SetRoadColorsEvent))

(fn ConstructionScript
  (bind _roadmesh (Variables|Default|GetRoadMesh))
  (Components|StaticMesh|SetStaticMesh _roadmesh (Variables|Default|GetRoadCustomMesh))
  (Rendering|Material|SetMaterial _roadmesh 0 "/Game/Materials/MI_RoadColor1.MI_RoadColor1")
  (Rendering|Material|SetMaterial _roadmesh 1 "/Game/Materials/MI_RoadColor2.MI_RoadColor2")
  (bind _returnvalue (Rendering|Material|CreateDynamicMaterialInstance _roadmesh 0 "/Game/Materials/MI_RoadColor1.MI_RoadColor1" "None" :!class /Script/Engine.PrimitiveComponent))
  (Variables|Default|SetDynMatColor1 _returnvalue)
  (bind _returnvalue_2 (Rendering|Material|CreateDynamicMaterialInstance _roadmesh 1 "/Game/Materials/MI_RoadColor2.MI_RoadColor2" "None" :!class /Script/Engine.PrimitiveComponent))
  (Variables|Default|SetDynMatColor2 _returnvalue_2))