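; BP_BallBroken is the broken-ball actor, made of separate shell and bottom pieces tinted to a ball color.
; The construction script creates one dynamic material instance from the first shell piece, and BeginPlay caches the GB_GameInstance.
; SetDestructibleColor applies that shared material to every piece, then sets its ColorPick parameter to one of the game instance's two colors based on ColorId.
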(event Custom|SetDestructibleColor
  (bind _gameinstanceref (Variables|Default|GetGameInstanceRef))
  (Rendering|Material|SetMaterial (Variables|Default|GetballBreakShell06) 0 (Variables|Default|GetDynMat))
  (if (Utilities|Enum|Equal(Enum) (Variables|Default|GetColorId) "NewEnumerator0")
    (Rendering|Material|SetVectorParameterValue (Variables|Default|GetDynMat) "ColorPick" (Variables|/Game/Blueprints/GB_GameInstance.GB_GameInstance_C|GetColor1 _gameinstanceref) :!class /Script/Engine.MaterialInstanceDynamic)
    (else
      (Rendering|Material|SetVectorParameterValue (Variables|Default|GetDynMat) "ColorPick" (Variables|/Game/Blueprints/GB_GameInstance.GB_GameInstance_C|GetColor2 _gameinstanceref) :!class /Script/Engine.MaterialInstanceDynamic))))

(event EventBeginPlay
  (bind _asgb_game_instance (Utilities|Casting|CastToGB_GameInstance (Game|GetGameInstance)))
  (Variables|Default|SetGameInstanceRef _asgb_game_instance))

(fn ConstructionScript
  (bind _ballbreakshell01 (Variables|Default|GetballBreakShell01))
  (bind _returnvalue (Rendering|Material|CreateDynamicMaterialInstance _ballbreakshell01 0 (Rendering|Material|GetMaterial _ballbreakshell01 0) "None" :!class /Script/Engine.PrimitiveComponent))
  (Variables|Default|SetDynMat _returnvalue))