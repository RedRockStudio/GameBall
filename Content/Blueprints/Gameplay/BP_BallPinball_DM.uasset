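; Destructible pinball ball Blueprint that tints its destructible component with one of two colors stored in the game instance.
; The construction script creates a dynamic material instance on the destructible's first material slot, and BeginPlay caches the GB_GameInstance reference.
; The SetDestructibleColor event writes Color1 or Color2 to that material's ColorPick parameter, depending on ColorId.
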(event Custom|SetDestructibleColor
  (bind _gameinstanceref (Variables|Default|GetGameInstanceRef))
  (if (Utilities|Enum|Equal(Enum) (Variables|Default|GetColorId) "NewEnumerator0")
    (Rendering|Material|SetVectorParameterValue (Variables|Default|GetDynMat3) "ColorPick" (Variables|/Game/Blueprints/GB_GameInstance.GB_GameInstance_C|GetColor1 _gameinstanceref) :!class /Script/Engine.MaterialInstanceDynamic)
    (else
      (Rendering|Material|SetVectorParameterValue (Variables|Default|GetDynMat3) "ColorPick" (Variables|/Game/Blueprints/GB_GameInstance.GB_GameInstance_C|GetColor2 _gameinstanceref) :!class /Script/Engine.MaterialInstanceDynamic))))

(event EventBeginPlay
  (bind _asgb_game_instance (Utilities|Casting|CastToGB_GameInstance (Game|GetGameInstance)))
  (Variables|Default|SetGameInstanceRef _asgb_game_instance))

(fn ConstructionScript
  (bind _destructible (Variables|Default|GetDestructible))
  (bind _returnvalue (Rendering|Material|CreateDynamicMaterialInstance _destructible 0 (Rendering|Material|GetMaterial _destructible 0) "None" :!class /Script/Engine.PrimitiveComponent))
  (Variables|Default|SetDynMat3 _returnvalue))