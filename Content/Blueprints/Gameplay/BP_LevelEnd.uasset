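; Level finish trigger with a slowly spinning finish circle that completes the level when a living BP_Ball overlaps its sphere.
; On the first valid overlap it updates level and color state on the GameInstance, saves, plays a win sound and resets the saved location.
; Fireworks spawn at three arrows, each randomly colored through a dynamic material instance.
; After a short delay it opens a level, or runs the all-levels-passed finale with slow motion and stopped camera.
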(event OnComponentBeginOverlap(Sphere)
  (params (OverlappedComponent :type Primitive%20Component%20Object%20Reference) (OtherActor :type Actor%20Object%20Reference) (OtherComp :type Primitive%20Component%20Object%20Reference) (OtherBodyIndex :type Integer) (bFromSweep :type Boolean) (SweepResult :type Hit%20Result%20Structure%20%28by%20ref%29))
  (bind _gameinstanceref (Variables|Default|GetGameInstanceRef))
  (bind _asbp_ball (Utilities|Casting|CastToBP_Ball OtherActor))
  (bind _output_get (Variables|Default|SetPlayerRef _asbp_ball))
  (if (not (Variables|/Game/Blueprints/Gameplay/BP_Ball.BP_Ball_C|GetisPlayerDead? _output_get))
    (Utilities|FlowControl|DoOnce false
      (:Completed
        (Utilities|FlowControl|Sequence
          (:then_0
            (Variables|/Game/Blueprints/GB_GameInstance.GB_GameInstance_C|SetColorSelectionActivated _gameinstanceref false)
            (Default|Level+1 _gameinstanceref)
            (Default|SelectColors _gameinstanceref)
            (Default|SaveGame _gameinstanceref)
            (Utilities|FlowControl|Delay 2.2)
            (if (Variables|/Game/Blueprints/GB_GameInstance.GB_GameInstance_C|GetisAllLevelsPassed? (Variables|Default|GetGameInstanceRef))
              (CallFunction|FinishAllFunc)
              (else
                (Default|OpenLevel _gameinstanceref))))
          (:then_1
            (Audio|PlaySound2D "/Game/Audio/SndFX/Win_Cue.Win_Cue" 1.0 1.0 0.0 0 0)
            (CallFunction|FireworksFunc)
            (if (not (Variables|/Game/Blueprints/GB_GameInstance.GB_GameInstance_C|GetisAllLevelsPassed? (Variables|Default|GetGameInstanceRef)))
              (Default|CallOnLevelComplete (Variables|Default|GetGameModeRef))))
          (:then_2
            (Variables|/Game/Blueprints/GB_GameInstance.GB_GameInstance_C|SetSavedLastLoc (Variables|Default|GetGameInstanceRef) "0, 0, 0")))))))

(event EventBeginPlay
  (bind _asgb_game_instance (Utilities|Casting|CastToGB_GameInstance (Game|GetGameInstance)))
  (Variables|Default|SetGameInstanceRef _asgb_game_instance)
  (bind _asgame_ball_gm (Utilities|Casting|CastTogameBallGM (Game|GetGameMode)))
  (Variables|Default|SetGameModeRef _asgame_ball_gm))

(event EventTick
  (params (DeltaSeconds :type Float%20%28single-precision%29))
  (Transformation|AddLocalRotation (Variables|Default|GetFinishCircle) (Math|Rotator|MakeRotator 0.0 0.0 (* DeltaSeconds 2.0)) false false))

(fn ConstructionScript)

(fn FinishAllFunc
  (bind _playerref (Variables|Default|GetPlayerRef))
  (Default|SloMoEvent _playerref)
  (Default|StopCamEvent _playerref)
  (Variables|/Game/Blueprints/Gameplay/BP_Ball.BP_Ball_C|SetisPlayerCanBeKilled? _playerref false)
  (Default|CallOnAllLevelsPassed (Variables|Default|GetGameModeRef))
  (Variables|/Game/Blueprints/GB_GameInstance.GB_GameInstance_C|SetisAllLevelsPassed? (Variables|Default|GetGameInstanceRef) false))

(fn FireworksFunc
  (bind _arrow1 (Variables|Default|GetArrow1))
  (bind _arrow2 (Variables|Default|GetArrow2))
  (bind _arrow3 (Variables|Default|GetArrow3))
  (bind _returnvalue (Transformation|GetWorldTransform _arrow3))
  (bind _returnvalue_2 (Transformation|GetWorldTransform _arrow1))
  (bind _returnvalue_3 (Transformation|GetWorldTransform _arrow2))
  (bind _returnvalue_4 (Effects|SpawnEmitteratLocation "/Game/Particles/P_Fireworks.P_Fireworks" (.location _returnvalue_2) (.rotation _returnvalue_2)))
  (CallFunction|FireworksColorSelectionFunc _returnvalue_4 _returnvalue_4)
  (bind _returnvalue_5 (Effects|SpawnEmitteratLocation "/Game/Particles/P_Fireworks.P_Fireworks" (.location _returnvalue_3) (.rotation _returnvalue_3)))
  (CallFunction|FireworksColorSelectionFunc _returnvalue_5 _returnvalue_5)
  (bind _returnvalue_6 (Effects|SpawnEmitteratLocation "/Game/Particles/P_Fireworks.P_Fireworks" (.location _returnvalue) (.rotation _returnvalue)))
  (CallFunction|FireworksColorSelectionFunc _returnvalue_6 _returnvalue_6))

(fn FireworksColorSelectionFunc
  (params (self2 :type Primitive%20Component%20Object%20Reference) (InputPin :type Particle%20System%20Component%20Object%20Reference))
  (bind _colourselection (Variables|Default|GetColourSelection))
  (bind _returnvalue (Rendering|Material|CreateDynamicMaterialInstance self2 3 "/Game/Materials/Masters/M_StarParticle.M_StarParticle" "None" :!class /Script/Engine.PrimitiveComponent))
  (Rendering|Material|SetVectorParameterValue _returnvalue "Colour" (Utilities|Array|Get(acopy) _colourselection (Math|Random|RandomIntegerinRange 0 (Utilities|Array|LastIndex _colourselection))) :!class /Script/Engine.MaterialInstanceDynamic)
  (Rendering|Material|SetMaterial InputPin 3 _returnvalue))