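; Player ball pawn for a mobile runner: a physics ball pushed forward by impulses, steered by touch swipes and pressed onto the surface by a downward trace.
; Its camera advances with timeline-eased speed while trailing boxes follow it, destroying passed cubes.
; The ball swaps between two GameInstance colors via a dynamic material and component tag.
; Death swaps in a destructible ball with slow motion; continue or restart saves its location.
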(event OnComponentBeginOverlap(BoxCleaner)
  (params (OverlappedComponent :type Primitive%20Component%20Object%20Reference) (OtherActor :type Actor%20Object%20Reference) (OtherComp :type Primitive%20Component%20Object%20Reference) (OtherBodyIndex :type Integer) (bFromSweep :type Boolean) (SweepResult :type Hit%20Result%20Structure%20%28by%20ref%29))
  ;[1 1 1] Cleaner and Ball Collision Wall Movement
  (bind _asbp_cube (Utilities|Casting|CastToBP_Cube OtherActor))
  (Actor|DestroyActor _asbp_cube))

(event Custom|Swipe
  (bind _returnvalue (Game|GetPlayerController 0))
  (bind _touchindex (Variables|Default|GetTouchIndex))
  (bind _swipespeed (Variables|Default|GetSwipeSpeed))
  (bind _ball (Variables|Default|GetBall))
  (bind (_locationx _locationy _biscurrentlypressed) (Class|PlayerController|GetInputTouchState _returnvalue _touchindex))
  ;[1 1 1] Swipe
  (if (not (or (Variables|Default|GetisPlayerDead?) (not (Variables|Default|GetisGameStarted?))))
    (if _biscurrentlypressed
      (if (Variables|Default|GetWasTouched?)
        (Utilities|IsValid _ball
          (:Is%20Valid
            (Physics|AddImpulse _ball (Math|Vector|MakeVector 0.0 (* (/ (- _locationx (Variables|Default|GetX)) _swipespeed) 1.0) 0.0) "None" true)
            (Physics|AddImpulse _ball (Math|Vector|MakeVector (* (/ (- _locationy (Variables|Default|GetY)) _swipespeed) -1.0) 0.0 0.0) "None" true)
            (Variables|Default|SetX _locationx)
            (Variables|Default|SetY _locationy)))
        (else
          (Variables|Default|SetWasTouched? true)
          (Variables|Default|SetX _locationx)
          (Variables|Default|SetY _locationy)))
      (else
        (Variables|Default|SetWasTouched? false)))))

(event Custom|ImpulseDown
  (params (DeltaSeconds :type Float%20%28single-precision%29))
  (bind _returnvalue (Transformation|GetActorLocation))
  ;[1 1 1] ImpulseDown
  (Utilities|IsValid (Variables|Default|GetBall)
    (:Is%20Valid
      (if (Variables|Default|GetisGameStarted?)
        (bind _outhit (Collision|LineTraceByChannel _returnvalue (- _returnvalue "0.000000, 0,500.000000") "TraceTypeQuery1" false 0 "None"))
        (Physics|AddImpulse (Variables|Default|GetBall) (* (* (.ImpactNormal (Collision|BreakHitResult _outhit)) -1) (* (Variables|Default|GetTableStickyness) DeltaSeconds)) "None" true)))))

(event Custom|ToContinueEvent
  (bind _gameinstanceref (Variables|Default|GetGameInstanceRef))
  ;[1 1 1] Continue and Restart
  (Variables|/Game/Blueprints/GB_GameInstance.GB_GameInstance_C|SetSavedLastLoc _gameinstanceref (.location (Variables|Default|GetBallWorldTransform)))
  (Variables|/Game/Blueprints/GB_GameInstance.GB_GameInstance_C|SetContinue? _gameinstanceref true))

(event Custom|SpawnParticlesEvents
  (bind _ball (Variables|Default|GetBall))
  (bind _returnvalue (Transformation|GetWorldLocation _ball))
  ;[1 1 1] Spawn Emitters
  (bind _returnvalue_2 (Effects|SpawnEmitterAttached "/Game/Particles/P_BallFX.P_BallFX" _ball "None" _returnvalue "0, 0, 0" "1.000000,1.000000,1.000000" "KeepWorldPosition"))
  (Variables|Default|SetP_BallFXRef _returnvalue_2)
  (bind _returnvalue_3 (Effects|SpawnEmitterAttached "/Game/Particles/P_Trail.P_Trail" _ball "None" _returnvalue "0, 0, 0" "1.000000,1.000000,1.000000" "KeepWorldPosition"))
  (Variables|Default|SetP_TrailRef _returnvalue_3))

(event Custom|SloMoEvent
  ;[0.4271 0.01046 0] PlayerDeath
  (bind _track1 (Timeline|SloMoOfDeath PlayFromStart) ; SloMo
    (:Update
      (Utilities|Time|SetGlobalTimeDilation _track1))))

(event Custom|StopCamEvent
  (bind _camera (Variables|Default|GetCamera))
  (bind _camera_2 (Variables|Default|GetCamera))
  ;[0.2387 0.7881 1] ImpulseForwardCamera
  (Utilities|FlowControl|Sequence
    (:then_0
      (Utilities|FlowControl|Gate false) ; enters at Close
    )
    (:then_1
      (Utilities|FlowControl|Gate true) ; enters at Open
    )))

(event Custom|CleanerBoxMove
  (bind _camera (Variables|Default|GetCamera))
  (bind _returnvalue (Transformation|GetWorldLocation _camera))
  ;[1 1 1] Cleaner and Ball Collision Wall Movement
  (Utilities|IsValid (Variables|Default|GetBall)
    (:Is%20Valid
      (Transformation|SetWorldLocation (Variables|Default|GetBoxCleaner) (Math|Vector|MakeVector (- (.x _returnvalue) (Variables|BallSettings|GetCleanerOffset)) 0.0 0.0) false false)
      (Transformation|SetWorldLocation (Variables|Default|GetBoxBallCollision) (Math|Vector|MakeVector (- (.x _returnvalue) (Variables|BallSettings|GetCollisionBoxOffset)) 0.0 0.0) false false)
      (Transformation|SetWorldLocation (Variables|Default|GetBoxBallCollision2) (Math|Vector|MakeVector (+ (.x _returnvalue) (Variables|BallSettings|GetCollisionBox2Offset)) 0.0 0.0) false false))))

(event Custom|ImpulseForward
  (bind _ball (Variables|Default|GetBall))
  ;[1 1 1] Impulse Forward
  (Utilities|IsValid _ball
    (:Is%20Valid
      (if (not (Variables|Default|GetisPlayerDead?))
        (Physics|AddImpulse _ball (Math|Vector|MakeVector (Variables|BallSettings|GetForwardPush) 0.0 0.0) "None" true)))))

(event Custom|SetPlayerColorEvent
  ;[1 1 1] SetColorEvent
  (Rendering|Material|SetVectorParameterValue (Variables|BallSettings|GetDynMat) "ColorPick" (Variables|/Game/Blueprints/GB_GameInstance.GB_GameInstance_C|GetColor1 (Variables|Default|GetGameInstanceRef)) :!class /Script/Engine.MaterialInstanceDynamic)
  (Variables|Default|SetColorIndex "NewEnumerator0")
  (|SetBy-RefVar (Utilities|Array|Get(acopy) (Variables|/Script/Engine.ActorComponent|GetComponentTags (Variables|Default|GetBall))) "Color1"))

(event Custom|TimerEvent
  ;[1 1 1] Timer
  (Utilities|FlowControl|Delay 1.0)
  (bind _output_get (Variables|Default|SetTimerCount (+ (Variables|Default|GetTimerCount) 1))))

(event Custom|PlayerDeathEvent
  (bind _ball (Variables|Default|GetBall))
  ;[0.4271 0.01046 0] PlayerDeath
  (Utilities|FlowControl|DoOnce false
    (:Completed
      (Utilities|FlowControl|Sequence
        (:then_0
          (Variables|Default|SetisPlayerDead? true)
          (Rendering|SetVisibility _ball false false)
          (Variables|Default|SetBallWorldTransform (Transformation|GetWorldTransform _ball))
          (Variables|Default|SetBallForwardVector (Math|Vector|GetForwardVector _ball))
          (Components|DestroyComponent _ball)
          (Effects|SpawnEmitteratLocation "/Game/Particles/P_BallExp.P_BallExp" (.location (Variables|Default|GetBallWorldTransform)))
          (Audio|PlaySound2D "/Game/Audio/SndFX/Death_Cue.Death_Cue" 1.0 1.0 0.0 0 0)
          (Game|Feedback|PlayDynamicForceFeedback (Game|GetPlayerController 0) 1.0 0.2 true true true true))
        (:then_1
          (bind _track1 (Timeline|SloMoOfDeath PlayFromStart) ; SloMo
            (:Update
              (Utilities|Time|SetGlobalTimeDilation _track1))))
        (:then_2
          (bind _returnvalue (Game|SpawnActorfromClass "/Game/Blueprints/Gameplay/BP_BallPinball_DM.BP_BallPinball_DM_C" (Variables|Default|GetBallWorldTransform) "Undefined" 0 0 :!pinned true)) ; SpawnDestractibleBall
          (bind _output_get (Variables|Default|SetBallDestrRef _returnvalue))
          (Variables|/Game/Blueprints/Gameplay/BP_BallPinball_DM.BP_BallPinball_DM_C|SetColorId _returnvalue (Variables|Default|GetColorIndex))
          (Default|SetDestructibleColor _output_get)
          (Physics|SetSimulatePhysics (Variables|/Game/Blueprints/Gameplay/BP_BallPinball_DM.BP_BallPinball_DM_C|GetDestructible _output_get) true)
          (Physics|AddImpulse (Variables|/Game/Blueprints/Gameplay/BP_BallPinball_DM.BP_BallPinball_DM_C|GetDestructible _output_get) (* (Variables|Default|GetBallForwardVector) 7.5e+02) "None" true)
          (Class|DestructibleComponent|ApplyRadiusDamage (Variables|/Game/Blueprints/Gameplay/BP_BallPinball_DM.BP_BallPinball_DM_C|GetDestructible _output_get) 1e+02 (.location (Variables|Default|GetBallWorldTransform)) 0.0 7.5e+03 true))))))

(event Custom|ImpulseForwardCamera
  (bind _camera (Variables|Default|GetCamera))
  (bind _camera_2 (Variables|Default|GetCamera))
  ;[0.2387 0.7881 1] ImpulseForwardCamera
  (Utilities|FlowControl|Sequence
    (:then_0
      (if (not (Variables|Default|GetisPlayerDead?))
        (Utilities|FlowControl|Gate false
          (:Exit
            (Utilities|FlowControl|Sequence :!pinned true ; MainImpulseToCam
              (:then_0
                (Transformation|AddRelativeLocation _camera_2 (Math|Vector|MakeVector (+ (.y (Transformation|GetWorldLocation _camera_2)) (Math|Float|Lerp 0.0 (/ (Variables|BallSettings|GetForwardPush) (Variables|Default|GetCamMoveValue)) (stale _trackofalpha))) 0.0 0.0) true false))
              (:then_1
                (Utilities|FlowControl|DoOnce false
                  (:Completed
                    (bind _trackofalpha (Timeline|TL_impulse PlayFromStart))))))))
        (else
          (Utilities|FlowControl|Sequence :!label _label
            (:then_0
              (Transformation|AddRelativeLocation _camera (Math|Vector|MakeVector (+ (.y (Transformation|GetWorldLocation _camera)) (Math|Float|Lerp (/ (Variables|BallSettings|GetForwardPush) (Variables|Default|GetCamMoveValue)) 0.0 (stale _trackofalpha_2))) 0.0 0.0) false false))
            (:then_1
              (Utilities|FlowControl|DoOnce false
                (:Completed
                  (bind _trackofalpha_2 (Timeline|TL_ImpulseToStop PlayFromStart)))))))))
    (:then_1
      (Utilities|FlowControl|Gate true
        (:Exit
          (goto _label))))))

(event Custom|ChangeColorEvent
  (bind _gameinstanceref (Variables|Default|GetGameInstanceRef))
  (bind _dynmat (Variables|BallSettings|GetDynMat))
  ;[0 0 0] DevBlock
  (Utilities|FlowControl|FlipFlop
    (:A
      (Rendering|Material|SetVectorParameterValue _dynmat "ColorPick" (Variables|/Game/Blueprints/GB_GameInstance.GB_GameInstance_C|GetColor2 _gameinstanceref) :!class /Script/Engine.MaterialInstanceDynamic)
      (Variables|Default|SetColorIndex "NewEnumerator1")
      (|SetBy-RefVar (Utilities|Array|Get(acopy) (Variables|/Script/Engine.ActorComponent|GetComponentTags (Variables|Default|GetBall))) "Color2")
      (Development|PrintString "SetPlayerColor" true true "(R=1.000000,G=1.000000,B=1.000000,A=1.000000)"))
    (:B
      (Rendering|Material|SetVectorParameterValue _dynmat "ColorPick" (Variables|/Game/Blueprints/GB_GameInstance.GB_GameInstance_C|GetColor1 _gameinstanceref) :!class /Script/Engine.MaterialInstanceDynamic)
      (Variables|Default|SetColorIndex "NewEnumerator0")
      (|SetBy-RefVar (Utilities|Array|Get(acopy) (Variables|/Script/Engine.ActorComponent|GetComponentTags (Variables|Default|GetBall))) "Color1")
      (Development|PrintString "SetPlayerColor" true true "(R=1.000000,G=1.000000,B=1.000000,A=1.000000)"))))

(event Custom|ToRestartEvent
  (bind _gameinstanceref (Variables|Default|GetGameInstanceRef))
  ;[1 1 1] Continue and Restart
  (Variables|/Game/Blueprints/GB_GameInstance.GB_GameInstance_C|SetSavedLastLoc _gameinstanceref (.location (Variables|Default|GetBallWorldTransform)))
  (Variables|/Game/Blueprints/GB_GameInstance.GB_GameInstance_C|SetRestart? _gameinstanceref true))

(event EventBeginPlay
  (Utilities|FlowControl|Sequence
    (:then_0
      (bind _asgb_game_instance (Utilities|Casting|CastToGB_GameInstance (Game|GetGameInstance)))
      (Variables|Default|SetGameInstanceRef _asgb_game_instance)
      (CallFunction|SetPlayerColorEvent)
      (CallFunction|SpawnLevelonRestart))
    (:then_1
      (bind _asgame_ball_gm (Utilities|Casting|CastTogameBallGM (Game|GetGameMode)))
      (bind _output_get (Variables|Default|SetGameModeRef _asgame_ball_gm))
      (EventDispatchers|BindEventtoOnPlayerDeath _output_get (EventDispatchers|CreateEvent :!event Custom|PlayerDeathEvent))
      (Default|ShowMainWidget (Variables|Default|GetGameModeRef))
      (Development|ExecuteConsoleCommand "stat fps" 0))
    (:then_2
      (bind _outactors (Actor|GetAllActorsOfClass "/Game/Blueprints/Gameplay/BP_LevelEnd.BP_LevelEnd_C"))
      (Variables|Default|SetLevelEndRef (Utilities|Array|Get(acopy) _outactors))
      (CallFunction|SpawnParticlesEvents))))

(event EventTick
  (params (DeltaSeconds :type Float%20%28single-precision%29))
  ;[1 1 1] EventTick
  (Utilities|FlowControl|Sequence
    (:then_0
      (CallFunction|Swipe)
      (CallFunction|ImpulseDown DeltaSeconds)
      (CallFunction|TimerEvent)
      (CallFunction|CleanerBoxMove))
    (:then_1
      (if (Variables|/Game/Blueprints/gameBallGM.gameBallGM_C|GetStartMoving (.AsGame%20Ball%20GM (Utilities|Casting|CastTogameBallGM (Game|GetGameMode))))
        (CallFunction|ImpulseForward)
        (CallFunction|ImpulseForwardCamera)
        (Utilities|FlowControl|DoOnce false
          (:Completed
            (Components|DestroyComponent (Variables|Default|GetP_Tap))
            (Physics|SetSimulatePhysics (Variables|Default|GetBall) true)
            (Variables|Default|SetisGameStarted? true)))))))

(event Input|KeyboardEvents|Z
  (params (Key :type Key%20Structure))
  ;[0 0 0] DevBlock
)

(event Input|TouchEvents|InputTouch
  (params (Location :type Vector) (FingerIndex :type ETouchIndex%20Enum))
  ;[1 1 1] Swipe
  (:Moved
    (Variables|Default|SetTouchIndex FingerIndex)))

(fn ConstructionScript
  (Utilities|FlowControl|Sequence
    (:then_0
      (bind _returnvalue (Rendering|Material|CreateDynamicMaterialInstance (Variables|Default|GetBall) 0 (Variables|BallSettings|GetInsMat) "None" :!class /Script/Engine.PrimitiveComponent))
      (Variables|BallSettings|SetDynMat _returnvalue))
    (:then_1)))

(fn BallColorSwitch
  (if (Components|ComponentHasTag (Variables|Default|GetBall) "Color1")
    (Rendering|Material|SetVectorParameterValue (Variables|BallSettings|GetDynMat) "ColorPick" (Variables|/Game/Blueprints/GB_GameInstance.GB_GameInstance_C|GetColor2 (Variables|Default|GetGameInstanceRef)) :!class /Script/Engine.MaterialInstanceDynamic)
    (Variables|Default|SetColorIndex "NewEnumerator1")
    (|SetBy-RefVar (Utilities|Array|Get(acopy) (Variables|/Script/Engine.ActorComponent|GetComponentTags (Variables|Default|GetBall))) "Color2")
    (else
      (Rendering|Material|SetVectorParameterValue (Variables|BallSettings|GetDynMat) "ColorPick" (Variables|/Game/Blueprints/GB_GameInstance.GB_GameInstance_C|GetColor1 (Variables|Default|GetGameInstanceRef)) :!class /Script/Engine.MaterialInstanceDynamic)
      (Variables|Default|SetColorIndex "NewEnumerator0")
      (|SetBy-RefVar (Utilities|Array|Get(acopy) (Variables|/Script/Engine.ActorComponent|GetComponentTags (Variables|Default|GetBall))) "Color1"))))

(fn SpawnLevelNumberTxt
  (Game|SpawnActorfromClass "/Game/Blueprints/Gameplay/BP_LvlNumber.BP_LvlNumber_C" (Math|Transform|MakeTransform (Math|Vector|MakeVector (+ (.x (Transformation|GetWorldLocation (Variables|Default|GetBall))) 1165.0) -1e+01 0.0) "0, 0, 0" "1,1,1") "AlwaysSpawn" 0 0))

(fn SpawnLevelonRestart
  (if (not (Variables|/Game/Blueprints/GB_GameInstance.GB_GameInstance_C|GetContinue? (Variables|Default|GetGameInstanceRef)))
    (CallFunction|SpawnLevelNumberTxt)))