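; Game instance for a level-based game that holds progress, settings and color palette across levels.
; Init loads or creates the GBSave slot, picks a random palette once, starts a session, then opens a level after a delay.
; Level helpers save before opening, advance zero-padded numeric level names and wrap to 0001 after the last.
; It also shows a cached loading-screen widget; AdsInitialize is empty, with its Appodeal setup left disconnected.
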(event Custom|ShowLoadingScrEvent
  (bind _returnvalue (Game|GetPlayerController 0))
  ;[1 1 1] Show Loading Scr
  (Utilities|IsValid (Variables|Default|GetLoadingScrWB)
    (:Is%20Valid
      _)
    (:Is%20Not%20Valid
      (bind _returnvalue_2 (UserInterface|CreateWidget "/Game/UI/LoadingScreen.LoadingScreen_C" _returnvalue))
      (Variables|Default|SetLoadingScrWB _returnvalue_2)))
  (UserInterface|Viewport|AddtoViewport (Variables|Default|GetLoadingScrWB) 0)
  (Variables|/Script/Engine.PlayerController|SetbShowMouseCursor _returnvalue true))

(event EventInit
  (CallFunction|SaveGameCheck)
  (CallFunction|SelectColors)
  (CallFunction|AdsInitialize)
  (Class|AnalyticsBlueprintLibrary|StartSession)
  (Utilities|FlowControl|Delay 1.5)
  (CallFunction|OpenLevel))

(fn SaveGameCheck
  (bind _returnvalue (SaveGame|DoesSaveGameExist (Variables|Default|GetGB_Save)))
  (if _returnvalue
    (CallFunction|LoadGame)
    (else
      (CallFunction|SaveGame))))

(fn SaveGame
  (Utilities|IsValid (Variables|Default|GetGB_SaveRef)
    (:Is%20Valid
      _)
    (:Is%20Not%20Valid
      (bind _returnvalue (SaveGame|CreateSaveGameObject "/Game/Blueprints/GB_Save.GB_Save_C"))
      (Variables|Default|SetGB_SaveRef _returnvalue)))
  (Variables|/Game/Blueprints/GB_Save.GB_Save_C|SetCurrLevel (Variables|Default|GetGB_SaveRef) (Variables|Save|GetCurrLevel))
  (Variables|/Game/Blueprints/GB_Save.GB_Save_C|SetisSoundOn? (Variables|Default|GetGB_SaveRef) (Variables|Save|GetisSndOn?))
  (Variables|/Game/Blueprints/GB_Save.GB_Save_C|SetisAdsRemoved? (Variables|Default|GetGB_SaveRef) (Variables|Save|GetisAdsRemoved?))
  (Variables|/Game/Blueprints/GB_Save.GB_Save_C|SetisVibrationOn? (Variables|Default|GetGB_SaveRef) (Variables|Save|GetisVibrationOn?))
  (SaveGame|SaveGametoSlot (Variables|Default|GetGB_SaveRef) (Variables|Default|GetGB_Save)))

(fn LoadGame
  (bind _returnvalue (SaveGame|LoadGamefromSlot (Variables|Default|GetGB_Save)))
  (bind _asgb_save (Utilities|Casting|CastToGB_Save _returnvalue))
  (Variables|Save|SetCurrLevel (Variables|/Game/Blueprints/GB_Save.GB_Save_C|GetCurrLevel _asgb_save))
  (Variables|Save|SetisSndOn? (Variables|/Game/Blueprints/GB_Save.GB_Save_C|GetisSoundOn? _asgb_save))
  (Variables|Save|SetisVibrationOn? (Variables|/Game/Blueprints/GB_Save.GB_Save_C|GetisVibrationOn? _asgb_save))
  (Variables|Save|SetisAdsRemoved? (Variables|/Game/Blueprints/GB_Save.GB_Save_C|GetisAdsRemoved? _asgb_save)))

(fn SelectColors
  (bind _colorsinfo (Variables|Colors|GetColorsInfo))
  (bind (_color1 _color2 _roadcolor1 _roadcolor2 _backcolor) (Utilities|Struct|BreakColorsStructure _colorsinfo))
  (if (Variables|Default|GetColorSelectionActivated)
    _
    (else
      (Variables|Colors|SetSelectedColorIndex (Math|Random|RandomIntegerinRange 0 (Utilities|Array|LastIndex (.Color1 (Utilities|Struct|BreakColorsStructure (Variables|Colors|GetColorsInfo))))))))
  (Variables|Default|SetColorSelectionActivated true)
  (Variables|Colors|SetColor1 (Utilities|Array|Get(acopy) _color1 (Variables|Colors|GetSelectedColorIndex)))
  (Variables|Colors|SetColor2 (Utilities|Array|Get(acopy) _color2 (Variables|Colors|GetSelectedColorIndex)))
  (Variables|Colors|SetRoadColor1 (Utilities|Array|Get(acopy) _roadcolor1 (Variables|Colors|GetSelectedColorIndex)))
  (Variables|Colors|SetRoadColor2 (Utilities|Array|Get(acopy) _roadcolor2 (Variables|Colors|GetSelectedColorIndex)))
  (Variables|Colors|SetBackColor (Utilities|Array|Get(acopy) _backcolor (Variables|Colors|GetSelectedColorIndex))))

(fn OpenLevel
  (CallFunction|SaveGame)
  (Game|OpenLevel(byName) (Variables|Save|GetCurrLevel)))

(fn Level+1
  (Variables|Default|SetCurrLevelString (Utilities|String|ToString(Integer) (+ (Math|Conversions|ToInteger(Byte) (Utilities|String|ToString(Name) (Variables|Save|GetCurrLevel))) 1)))
  (if (== (Utilities|String|Len (Variables|Default|GetCurrLevelString)) 1)
    (Variables|Save|SetCurrLevel (Utilities|String|StringToName (Utilities|String|Append (Utilities|String|MakeLiteralString "000") (Variables|Default|GetCurrLevelString))))
    (elif (== (Utilities|String|Len (Variables|Default|GetCurrLevelString)) 2)
      (Variables|Save|SetCurrLevel (Utilities|String|StringToName (Utilities|String|Append (Utilities|String|MakeLiteralString "00") (Variables|Default|GetCurrLevelString))))
      (elif (== (Utilities|String|Len (Variables|Default|GetCurrLevelString)) 3)
        (Variables|Save|SetCurrLevel (Utilities|String|StringToName (Utilities|String|Append (Utilities|String|MakeLiteralString "0") (Variables|Default|GetCurrLevelString))))
        (else
          (Variables|Save|SetCurrLevel (Utilities|String|StringToName (Variables|Default|GetCurrLevelString)))))))
  (CallFunction|LastLevelCheck))

(fn LastLevelCheck
  (if (> (Math|Conversions|ToInteger(Byte) (Utilities|String|ToString(Name) (Variables|Save|GetCurrLevel))) (Variables|Default|GetLastLevelNumber))
    (Variables|Default|SetisAllLevelsPassed? true)
    (Variables|Save|SetCurrLevel "0001")))

(fn AdsInitialize)